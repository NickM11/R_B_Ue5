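; AI controller for the Circle NPC that runs BT_CircleNPC on BeginPlay and feeds perception results into its Blackboard.
; Sight stimuli from the player set TargetActor, or clear it and store LastKnownLocation when sight is lost.
; Hearing stimuli from any source write their position to TargetLocation.
; OutOfRadius writes the supplied flag to IsInRadius, with no caller in this asset.
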(event OnTargetPerceptionUpdated(AIPerception)
  (params (Actor :type Actor%20Object%20Reference) (Stimulus :type AI%20Stimulus%20Structure))
  (CallFunction|HandleSightSense Actor Stimulus)
  (CallFunction|HandleSoundSense Stimulus))

(event EventBeginPlay
  (AI|RunBehaviorTree "/Game/HW10/AI/BT_CircleNPC.BT_CircleNPC"))

(event EventTick
  (params (DeltaSeconds :type Float%20%28single-precision%29)))

(fn ConstructionScript)

(fn HandleSightSense
  (params (Actor :type Actor%20Object%20Reference) (Stimulus :type AI%20Stimulus%20Structure))
  (Variables|Default|SetActor Actor)
  (bind _output_get (Variables|Default|SetStimulus Stimulus))
  (bind _returnvalue (Class|AIPerceptionSystem|GetSenseClassforStimulus _output_get))
  (if (== _returnvalue "/Script/AIModule.AISense_Sight")
    (if (== (Variables|Default|GetActor) (Game|GetPlayerCharacter 0))
      (AI|Components|Blackboard|SetValueasObject (Variables|Default|GetBlackboard) (Utilities|Name|MakeLiteralName "TargetActor") (Utilities|SelectObject (Game|GetPlayerCharacter 0) 0 (.bsuccessfullysensed (Variables|Default|GetStimulus))))
      (if (not (.bsuccessfullysensed (Variables|Default|GetStimulus)))
        (AI|Components|Blackboard|SetValueasVector (Variables|Default|GetBlackboard) (Utilities|Name|MakeLiteralName "LastKnownLocation") (.stimuluslocation (Variables|Default|GetStimulus))))
      (else
        (return)))
    (else
      (return))))

(fn OutOfRadius
  (params (IsInRadius :type Boolean))
  (AI|Components|Blackboard|SetValueasBool (Variables|Default|GetBlackboard) (Utilities|Name|MakeLiteralName "IsInRadius") IsInRadius))

(fn HandleSoundSense
  (params (Stimulus :type AI%20Stimulus%20Structure))
  (bind _returnvalue (Class|AIPerceptionSystem|GetSenseClassforStimulus Stimulus))
  (if (== _returnvalue "/Script/AIModule.AISense_Hearing")
    (AI|Components|Blackboard|SetValueasVector (Variables|Default|GetBlackboard) (Utilities|Name|MakeLiteralName "TargetLocation") (.StimulusLocation (Utilities|Struct|BreakAIStimulus (Variables|Default|GetStimulus))))))