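; Player character Blueprint that handles movement and mouse look and puts a health widget on screen.
; On BeginPlay it creates WB_Health for player controller 0, stores it and adds it to the viewport, with no health logic in this graph.
; Enhanced Input move and look actions call Move and Aim, which apply movement along the actor's forward and right vectors and add controller yaw and pitch.
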(event Input|EnhancedActionEvents|EnhancedInputActionIA_Move
  (params (ActionValue :type Vector%202D%20Structure) (ElapsedSeconds :type Float%20%28double-precision%29) (TriggeredSeconds :type Float%20%28double-precision%29) (InputAction :type Input%20Action%20Object%20Reference :default "/Game/Input/IA_Move.IA_Move"))
  (CallFunction|Move (.x ActionValue) (.y ActionValue)))

(event Input|EnhancedActionEvents|EnhancedInputActionIA_MouseLook
  (params (ActionValue :type Vector%202D%20Structure) (ElapsedSeconds :type Float%20%28double-precision%29) (TriggeredSeconds :type Float%20%28double-precision%29) (InputAction :type Input%20Action%20Object%20Reference :default "/Game/Input/IA_MouseLook.IA_MouseLook"))
  (CallFunction|Aim (.x ActionValue) (.y ActionValue)))

(event EventBeginPlay
  (bind _returnvalue (UserInterface|CreateWidget "/Game/HW8/WB_Health.WB_Health_C" (Game|GetPlayerController 0)))
  (bind _output_get (Variables|Default|SetHealthWidget _returnvalue))
  (UserInterface|Viewport|AddtoViewport _output_get 0))

(event Collision|EventActorBeginOverlap
  (params (OtherActor :type Actor%20Object%20Reference)))

(event EventTick
  (params (DeltaSeconds :type Float%20%28single-precision%29)))

(fn ConstructionScript)

(fn Move
  (params (Left%20/%20Right :type Float%20%28double-precision%29) (Forward%20/%20Backward :type Float%20%28double-precision%29))
  (Pawn|Input|AddMovementInput (Transformation|GetActorRightVector) Left%20/%20Right false)
  (Pawn|Input|AddMovementInput (Transformation|GetActorForwardVector) Forward%20/%20Backward false))

(fn Aim
  (params (Yaw :type Float%20%28double-precision%29) (Pitch :type Float%20%28double-precision%29))
  (Pawn|Input|AddControllerYawInput Yaw)
  (Pawn|Input|AddControllerPitchInput Pitch))