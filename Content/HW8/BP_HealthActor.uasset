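; BP_HealthActor is a health pickup that moves in a circle and adds health to the player character.
; Tick advances an angle by speed and sets the relative location using sine and cosine, scaling Center plus the trig term by Radius.
; Any Box overlap adds a fixed amount to the player reference cached at BeginPlay, without checking the overlapping actor or removing the pickup.
; The node capturing Center from the actor's location is unconnected.
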(event OnComponentBeginOverlap(Box)
  (params (OverlappedComponent :type Primitive%20Component%20Object%20Reference) (OtherActor :type Actor%20Object%20Reference) (OtherComp :type Primitive%20Component%20Object%20Reference) (OtherBodyIndex :type Integer) (bFromSweep :type Boolean) (SweepResult :type Hit%20Result%20Structure%20%28by%20ref%29))
  (bind _characterref (Variables|Default|GetCharacterRef))
  (Variables|/Game/HW8/BP_PlayableCharacter.BP_PlayableCharacter_C|SetHealth _characterref (+ (Variables|/Game/HW8/BP_PlayableCharacter.BP_PlayableCharacter_C|GetHealth _characterref) 2e+01)))

(event EventBeginPlay
  (bind _asbp_playable_character (Utilities|Casting|CastToBP_PlayableCharacter (Game|GetPlayerCharacter 0)))
  (Variables|Default|SetCharacterRef _asbp_playable_character))

(event Collision|EventActorBeginOverlap
  (params (OtherActor :type Actor%20Object%20Reference)))

(event EventTick
  (params (DeltaSeconds :type Float%20%28single-precision%29))
  (bind _center (Variables|Default|GetCenter))
  (Variables|Default|SetAngle (+ (* DeltaSeconds (Variables|Default|GetSpeed)) (Variables|Default|GetAngle)))
  (Transformation|SetActorRelativeLocation (Math|Vector|MakeVector (.x (Math|Vector|MakeVector (* (+ (.x _center) (Math|Trig|Cos(Degrees) (Variables|Default|GetAngle))) (Variables|Default|GetRadius)) (* (+ (.y _center) (Math|Trig|Sin(Degrees) (Variables|Default|GetAngle))) (Variables|Default|GetRadius)) (.z _center))) (.y (Math|Vector|MakeVector (* (+ (.x _center) (Math|Trig|Cos(Degrees) (Variables|Default|GetAngle))) (Variables|Default|GetRadius)) (* (+ (.y _center) (Math|Trig|Sin(Degrees) (Variables|Default|GetAngle))) (Variables|Default|GetRadius)) (.z _center))) (.z (Math|Vector|MakeVector (* (+ (.x _center) (Math|Trig|Cos(Degrees) (Variables|Default|GetAngle))) (Variables|Default|GetRadius)) (* (+ (.y _center) (Math|Trig|Sin(Degrees) (Variables|Default|GetAngle))) (Variables|Default|GetRadius)) (.z _center))))))

(fn ConstructionScript)