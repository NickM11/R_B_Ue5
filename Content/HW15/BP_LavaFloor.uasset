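; BP_LavaFloor is a lava hazard that applies damage over time to characters touching its LavaCollider.
; On overlap begin, it gets a character reference through CharRefMessage, sets that character's received damage, then calls StartDoT and DoT on it.
; On overlap end, it calls EndDot on the character.
; A separate DoPlayerDamge function sends a fixed DamageMessage to CharRef but is not called within this Blueprint.
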(event OnComponentBeginOverlap(Lavacollider)
  (params (OverlappedComponent :type Primitive%20Component%20Object%20Reference) (OtherActor :type Actor%20Object%20Reference) (OtherComp :type Primitive%20Component%20Object%20Reference) (OtherBodyIndex :type Integer) (bFromSweep :type Boolean) (SweepResult :type Hit%20Result%20Structure%20%28by%20ref%29))
  (bind _characterref (Class|BPICharacterRef|CharRef(Message) OtherActor))
  (Utilities|IsValid _characterref
    (:Is%20Valid
      (Variables|/Game/FirstPerson/Blueprints/BP_FirstPersonCharacter.BP_FirstPersonCharacter_C|SetDamageRecieved _characterref 2e+01)
      (Default|StartDoT _characterref)
      (Default|DoT _characterref))))

(event OnComponentEndOverlap(Lavacollider)
  (params (OverlappedComponent :type Primitive%20Component%20Object%20Reference) (OtherActor :type Actor%20Object%20Reference) (OtherComp :type Primitive%20Component%20Object%20Reference) (OtherBodyIndex :type Integer))
  (bind _characterref (Class|BPICharacterRef|CharRef(Message) OtherActor))
  (Utilities|IsValid _characterref
    (:Is%20Valid
      (Default|EndDot _characterref))))

(event EventBeginPlay)

(event Collision|EventActorBeginOverlap
  (params (OtherActor :type Actor%20Object%20Reference)))

(event EventTick
  (params (DeltaSeconds :type Float%20%28single-precision%29)))

(fn ConstructionScript)

(fn DoPlayerDamge
  (params (OverlappedPlayer :type Actor%20Object%20Reference))
  (Class|BPIDamage|Damage(Message) (Variables|Default|GetCharRef) 12.0))