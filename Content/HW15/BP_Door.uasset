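; BP_Door is a sliding door that moves on an Interact event and shows a widget when something is nearby.
; Interact plays a timeline that lerps the Door's relative X position, then reverses it after a short delay to slide it back.
; Box overlap begin and end toggle the Widget's visibility without filtering the overlapping actor.
; BeginPlay also creates a WB_InteractButton and stores it, but this graph never uses it.
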(event OnComponentBeginOverlap(Box)
  (params (OverlappedComponent :type Primitive%20Component%20Object%20Reference) (OtherActor :type Actor%20Object%20Reference) (OtherComp :type Primitive%20Component%20Object%20Reference) (OtherBodyIndex :type Integer) (bFromSweep :type Boolean) (SweepResult :type Hit%20Result%20Structure%20%28by%20ref%29))
  (Rendering|SetVisibility (Variables|Default|GetWidget) true false))

(event OnComponentEndOverlap(Box)
  (params (OverlappedComponent :type Primitive%20Component%20Object%20Reference) (OtherActor :type Actor%20Object%20Reference) (OtherComp :type Primitive%20Component%20Object%20Reference) (OtherBodyIndex :type Integer))
  (Rendering|SetVisibility (Variables|Default|GetWidget) false false))

(event EventBeginPlay
  (bind _returnvalue (UserInterface|CreateWidget "/Game/HW12_13/WB_InteractButton.WB_InteractButton_C"))
  (Variables|Default|SetInteractButtonRef _returnvalue))

(event Collision|EventActorBeginOverlap
  (params (OtherActor :type Actor%20Object%20Reference)))

(event EventTick
  (params (DeltaSeconds :type Float%20%28single-precision%29)))

(event EventInteract
  (bind _newtrack_0 (Timeline|Timeline Play)
    (:Update
      (Transformation|SetRelativeLocation (Variables|Default|GetDoor) (Math|Vector|MakeVector (Math|Float|Lerp -3.2e+02 2.4e+02 _newtrack_0) 0.0 0.0) false false))
    (:Finished
      (Utilities|FlowControl|Delay 3.0)
      (Timeline|Timeline Reverse))))

(fn ConstructionScript)