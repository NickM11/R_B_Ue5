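; BP_Player is a player Blueprint that lets input trigger actor spawning through the custom game mode.
; On BeginPlay it adds the IMC_Default Enhanced Input mapping context to its player controller, then caches the BP_CustomGamemode reference.
; The IA_SpawnActor input action prints a debug string and calls SpawnActor on that game mode, which owns the spawn logic.
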(event Input|EnhancedActionEvents|EnhancedInputActionIA_SpawnActor
  (params (ActionValue :type Boolean) (ElapsedSeconds :type Float%20%28double-precision%29) (TriggeredSeconds :type Float%20%28double-precision%29) (InputAction :type Input%20Action%20Object%20Reference :default "/Game/Input/IA_SpawnActor.IA_SpawnActor"))
  (Development|PrintString "Hello")
  (Default|SpawnActor (Variables|Default|GetAs%20BP%20Custom%20Gamemode)))

(event EventBeginPlay
  (bind _asplayer_controller (Utilities|Casting|CastToPlayerController (Pawn|GetController)))
  (Input|AddMappingContext (PlayerController|LocalPlayerSubsystems|GetEnhancedInputLocalPlayerSubsystem _asplayer_controller) "/Game/Input/IMC_Default.IMC_Default" 0 "(bIgnoreAllPressedKeysUntilRelease=True,bForceImmediately=False,bNotifyUserSettings=False)")
  (bind _asbp_custom_gamemode (Utilities|Casting|CastToBP_CustomGamemode (Game|GetGameMode)))
  (Variables|Default|SetAs%20BP%20Custom%20Gamemode _asbp_custom_gamemode))

(event Collision|EventActorBeginOverlap
  (params (OtherActor :type Actor%20Object%20Reference)))

(event EventTick
  (params (DeltaSeconds :type Float%20%28single-precision%29)))

(event Input|KeyboardEvents|F
  (params (Key :type Key%20Structure :default "None")))

(fn ConstructionScript)